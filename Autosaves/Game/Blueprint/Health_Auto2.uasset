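; Health Blueprint with TakeDamage, Heal and Die functions for tracking damage, healing and death, currently non-functional.
; All three functions have empty bodies, as the damage and heal logic is disconnected from the function entries.
; The unwired damage logic computes Amount minus CurrentHealth and calls Die when the result is zero or above, reversing the usual subtraction and death test.
; The unwired heal logic adds Amount, capping at MaxHealth unless CanOverHeal is set.
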(fn `Die`)

(fn `Heal`
  (params (Amount :type "Float (double-precision)") (CanOverHeal :type Boolean)))

(fn `TakeDamage`
  (params (Amount :type "Float (double-precision)")))