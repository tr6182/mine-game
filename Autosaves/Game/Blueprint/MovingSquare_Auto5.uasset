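; MovingSquare is an actor that moves toward the first player's pawn while IsChasingPlayer is true.
; Each Tick adds the normalized direction to the pawn, multiplied by Speed, to its location with a swept SetActorLocation.
; The step is not scaled by delta time, so movement depends on frame rate.
; When not chasing, it prints a NotMoving debug string every frame.
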(event `self.ReceiveTick`
  (params (DeltaSeconds :type "Float (single-precision)"))
  (if (`self.Is Chasing Player`)
    (`self.K2_SetActorLocation` (+ (`self.K2_GetActorLocation`) (* (`KismetMathLibrary.Normal` (- (`self.K2_GetActorLocation` (`GameplayStatics.GetPlayerPawn` 0)) (`self.K2_GetActorLocation`))) (`self.Speed`))) true)
    (else
      (`KismetSystemLibrary.PrintString` (`self.Not Moving`)))))

(fn `UserConstructionScript`)