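; Health component that tracks its owning actor's current health through damage and healing.
; TakeDamage subtracts from CurrentHealth and calls Die at zero or below, which destroys the owner.
; Heal adds health and caps it at MaxHealth unless overheal is allowed.
; BeginPlay creates and caches a HealthBar widget for the first player controller, but never displays it, and UpdateUI is an empty stub.
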(event `self.ReceiveBeginPlay`
  (bind _returnvalue (`|CreateWidget` "/Game/UI/HealthBar.HealthBar_C" (`GameplayStatics.GetPlayerController` 0)))
  (set `self.HealthBarCache` _returnvalue))

(fn `Die`
  ;[1 1 1] destroy actor this component is own by
  (`Actor.K2_DestroyActor` (`self.GetOwner`)))

(fn `Heal`
  (params (Amount :type "Float (double-precision)") (CanOverHeal :type Boolean))
  ;[1 1 1] Change health value
  (set `self.CurrentHealth` (+ (`self.CurrentHealth`) Amount))
  ;[1 1 1] Prevents overheal
  (if (not CanOverHeal)
    (set `self.CurrentHealth` (`KismetMathLibrary.FMin` (`self.CurrentHealth`) (`self.MaxHealth`)))))

(fn `TakeDamage`
  (params (Amount :type "Float (double-precision)"))
  ;[1 1 1] health value update
  (set `self.CurrentHealth` (- (`self.CurrentHealth`) Amount))
  ;[1 1 1] Check for death
  (if (<= (`self.CurrentHealth`) 0.0)
    (`self.Die`)))

(fn `UpdateUI`)